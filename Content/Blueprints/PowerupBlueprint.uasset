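; A powerup pickup, shown by a star mesh, that grants the player either a jump boost or a speed boost.
; On Begin Play it calls OnGenerate, defined outside these graphs, then sets the star's material to match the powerup type.
; On pickup it prints a message and overwrites the first player character's jump velocity or max walk speed, with no revert here.
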(event EventBeginPlay
  ;[1 1 1] On Begin Play, call the OnGenerate function to generate the Powerup, then check whether the Powerup is a JUMPBOOST or a SPEEDBOOST and assign the materials accordingly.
  (Class|Powerup|OnGenerate)
  (if (Utilities|Enum|Equal(Enum) (Variables|Default|GetPowerup) "JUMPBOOST")
    (Rendering|Material|SetMaterial (Variables|Default|Getstar) 0 "/Game/Materials/GreenMaterial.GreenMaterial")
    (elif (Utilities|Enum|Equal(Enum) (Variables|Default|GetPowerup) "SPEEDBOOST")
      (Rendering|Material|SetMaterial (Variables|Default|Getstar) 0 "/Game/Materials/WeaponRarityMaterials/LegendaryMaterial.LegendaryMaterial"))))

(event EventOnPickup
  (params (ActorThatPickedUp :type Actor%20Object%20Reference))
  ;[1 1 1] On pickup, check if powerup is a JUMPBOOST or a SPEEDBOOST
  (if (Utilities|Enum|Equal(Enum) (Variables|Default|GetPowerup) "JUMPBOOST")
    ;[1 1 1] If the powerup is a JUMPBOOST, print a string, then set the JumpZVelocity on the CharacterMovement to be equal to the value of JumpBoostHeight (700.0f)
    (Development|PrintString "JUMP BOOST ACTIVATED" true true "(R=0.000000,G=1.000000,B=0.033423,A=1.000000)")
    (Variables|/Script/Engine.CharacterMovementComponent|SetJumpZVelocity (Variables|/Script/Engine.Character|GetCharacterMovement (Game|GetPlayerCharacter 0)) (Variables|Default|GetJumpBoostHeight))
    (else
      ;[1 1 1] If the branch node returns FALSE (which means it is a SPEEDBOOST), print a string, then set the MaxWalkSpeed to be equal to SpeedBoostWalkSpeed (1350.0f)
      (Development|PrintString "SPEED BOOST ACTIVATED" true true "(R=1.000000,G=0.954921,B=0.000000,A=1.000000)")
      (Variables|/Script/Engine.CharacterMovementComponent|SetMaxWalkSpeed (Variables|/Script/Engine.Character|GetCharacterMovement (Game|GetPlayerCharacter 0)) (Variables|Default|GetSpeedBoostWalkSpeed)))))

(fn ConstructionScript)