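; EnemyCharacterBT is an enemy character Blueprint with AI perception and a child-actor gun, its name suggesting Behavior Tree control.
; Its Fire event forwards a direction to the GunBlueprint child actor, then rotates the character to face that direction.
; The perception update handler loops through each updated actor's last sensed stimuli checking for a "Noise" tag, but takes no action on a match.
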(event Custom|OnPerceptionUpdated_Event_0
  (params (UpdatedActors :type Array%20of%20Actor%20Object%20References))
  (for _array_element UpdatedActors
    (bind _info (Class|AIPerceptionComponent|GetActorsPerception (Variables|Default|GetAIPerception) _array_element))
    (for _array_element_2 (.lastsensedstimuli _info)
      (if (Utilities|Name|Equal(Name) (.Tag (Utilities|Struct|BreakAIStimulus _array_element_2)) "Noise")
        _))))

(event EventBeginPlay)

(event Collision|EventActorBeginOverlap
  (params (OtherActor :type Actor%20Object%20Reference)))

(event EventTick
  (params (DeltaSeconds :type Float%20%28single-precision%29)))

(event EventFire
  (params (FireDirection :type Vector :default "0, 0, 0"))
  (bind _asgun_blueprint (Utilities|Casting|CastToGunBlueprint (Variables|/Script/Engine.ChildActorComponent|GetChildActor (Variables|Default|GetGun))))
  (Default|Fire _asgun_blueprint FireDirection)
  (Transformation|SetActorRotation (Math|Conversions|RotationFromXVector FireDirection)))

(fn ConstructionScript)