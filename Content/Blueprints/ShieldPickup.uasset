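; Shield pickup that grants shield points to the actor that picks it up.
; BeginPlay calls OnGenerate, then sets the shield mesh material to match its small, medium or large ShieldType.
; OnPickup searches the actor's components for a HealthComponent and, if its shield is below maximum, adds the pickup's CurrentShield without clamping.
; Debug prints report the amount added or that shields are maxed.
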(event EventBeginPlay
  (Class|ShieldPickup|OnGenerate)
  (switch Utilities|FlowControl|Switch|SwitchonShieldType (Variables|Default|GetShieldType)
    (:SMALL
      (Rendering|Material|SetMaterial (Variables|Default|GetShield_fbx) 0 "/Game/Materials/GreenMaterial.GreenMaterial"))
    (:MEDIUM
      (Rendering|Material|SetMaterial (Variables|Default|GetShield_fbx) 0 "/Game/Materials/WeaponRarityMaterials/RareMaterial.RareMaterial"))
    (:LARGE
      (Rendering|Material|SetMaterial (Variables|Default|GetShield_fbx) 0 "/Game/Materials/WeaponRarityMaterials/LegendaryMaterial.LegendaryMaterial"))))

(event EventOnPickup
  (params (ActorThatPickedUp :type Actor%20Object%20Reference))
  (for _array_element (Actor|GetComponentsByClass ActorThatPickedUp "/Script/Engine.ActorComponent")
    (bind _ashealth_component (Utilities|Casting|CastToHealthComponent _array_element))
    (if (< (Variables|/Script/AdvGamesProgramming.HealthComponent|GetCurrentShield _ashealth_component) (Variables|/Script/AdvGamesProgramming.HealthComponent|GetMaxShield _ashealth_component))
      (Variables|/Script/AdvGamesProgramming.HealthComponent|SetCurrentShield _ashealth_component (+ (Variables|Default|GetCurrentShield) (Variables|/Script/AdvGamesProgramming.HealthComponent|GetCurrentShield _ashealth_component)))
      (Development|PrintString (Utilities|String|ToString(Integer) (Variables|Default|GetCurrentShield)))
      (else
        (Development|PrintString "Max Shields")))))

(fn ConstructionScript)